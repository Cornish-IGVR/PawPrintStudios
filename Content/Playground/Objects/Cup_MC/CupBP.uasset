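; CupBP is a grabbable cup prop that returns itself to a set spot after moving fast.
; BeginPlay gives the Grabable component a fixed grab on the static mesh, with the same transform for both hands and a hand animation.
; Tick checks the mesh's speed and, above a threshold, waits briefly, then teleports the actor to a hardcoded location.
; Comments mentioning a ring toss and inverted motion log labels suggest reused logic.
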(event EventBeginPlay
  (bind _returnvalue (Math|Transform|MakeTransform "1.100000,0.000000,-1.000000" "87.000000,320.000000,132.000000"))
  ;[1 1 1] Align Ring
  (Default|SetFixedGrab (Variables|Default|GetGrabable) (Variables|Default|GetStaticMesh) _returnvalue "/Game/Framework/Hands/Model/Animations/Grabs/hand_lighter.hand_lighter" _returnvalue))

(event EventTick
  (params (DeltaSeconds :type Float%20%28single-precision%29))
  ;[1 1 1] Is RingToss In Motion - If so, teleport to last location
  (if (> (Math|Vector|VectorLength (Transformation|GetComponentVelocity (Variables|Default|GetStaticMesh))) 2e+02)
    (Development|PrintString "Not Moving" false true "(R=0.000000,G=0.660000,B=1.000000,A=1.000000)" 1e+01)
    (Utilities|FlowControl|Delay 2.0)
    (Transformation|SetActorLocation "-290.000000,210.000000,390.000000" false true)
    (else
      (Development|PrintString "Moving" false true "(R=0.000000,G=0.660000,B=1.000000,A=1.000000)" 1e+01))))

(fn ConstructionScript)