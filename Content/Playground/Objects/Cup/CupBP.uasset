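; CupBP is a cup object that can be grabbed with either hand.
; On BeginPlay it gives its Grabable component a fixed grab on the static mesh, with identical left and right transforms and the Hand_lighter animation.
; A Hit handler, labelled as a ring-motion check, applies a zero impulse to moving components and otherwise logs "Not Moving" without showing it on screen.
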(event EventBeginPlay
  (bind _returnvalue (Math|Transform|MakeTransform "1.100000,0.000000,-10.000000" "87.000000,320.000000,132.000000"))
  (Default|SetFixedGrab (Variables|Default|GetGrabable) (Variables|Default|GetStaticMesh) _returnvalue "/Game/Framework/Hands/Model/Animations/Grabs/hand_lighter.hand_lighter" _returnvalue))

(event EventTick
  (params (DeltaSeconds :type Float%20%28single-precision%29))
  ;[1 1 1] Is Ring In Motion
)

(event Collision|EventHit
  (params (MyComp :type Primitive%20Component%20Object%20Reference) (Other :type Actor%20Object%20Reference) (OtherComp :type Primitive%20Component%20Object%20Reference) (bSelfMoved :type Boolean) (HitLocation :type Vector :default "0, 0, 0") (HitNormal :type Vector :default "0, 0, 0") (NormalImpulse :type Vector :default "0, 0, 0") (Hit :type Hit%20Result%20Structure%20%28by%20ref%29))
  ;[1 1 1] Is Ring In Motion
  (if (> (Math|Vector|VectorLength (Transformation|GetComponentVelocity OtherComp)) 0.0)
    (Physics|AddImpulseatLocation OtherComp "0, 0, 0" (Transformation|GetActorLocation) "None")
    (else
      (Development|PrintString "Not Moving" false true "(R=0.000000,G=0.660000,B=1.000000,A=1.000000)" 1e+01))))

(fn ConstructionScript)